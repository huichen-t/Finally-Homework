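; Moving platform with sliding rail doors that shuttles between its origin and a configurable end location and rotation, with motor, steam and tone audio.
; Travel, rotation and door timelines drive lerps; each finished trip opens the doors, waits, then departs the opposite way.
; Safety colliders reverse an active trip or reopen moving doors when a BP_Char_Master overlaps.
; Construction script previews the end or midpoint pose in the editor.
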(event OnComponentBeginOverlap(SafetyCollider)
  (params (OverlappedComponent :type Primitive%20Component%20Object%20Reference) (OtherActor :type Actor%20Object%20Reference) (OtherComp :type Primitive%20Component%20Object%20Reference) (OtherBodyIndex :type Integer) (bFromSweep :type Boolean) (SweepResult :type Hit%20Result%20Structure%20%28by%20ref%29))
  (bind _platform_travel_timeline (Variables|Default|GetPlatform%20Travel%20Timeline))
  ;[1 1 1] Reverses Direction if collision occurs with Actor
  (Utilities|Casting|CastToBP_Char_Master OtherActor)
  (if (Components|Activation|IsActive _platform_travel_timeline)
    (if (Class|TimelineComponent|IsReversing _platform_travel_timeline)
      (Utilities|FlowControl|Sequence
        (:then_0
          ;[1 1 1] Sets End Location and Rotation- Stop Delay- Reversing
          (bind (_direction _platform_travel) (Timeline|Platform%20Travel%20Timeline Play) ; Float Translation Curve
            (:Update
              (Utilities|FlowControl|Sequence
                (:then_1
                  (Transformation|SetRelativeLocation (Variables|Default|GetPlatform) (Math|Vector|Lerp(Vector) "0, 0, 0" (Variables|PlatformControls|GetEndLocation) _platform_travel) false false))))
            (:Finished
              (Utilities|FlowControl|Sequence
                (:then_0
                  (Utilities|FlowControl|Delay (Variables|PlatformControls|GetStopDelay))
                  (Utilities|FlowControl|Sequence
                    (:then_0
                      ;[1 1 1] Start/Play/Stop Audio
                      (Audio|Components|Audio|Play (Variables|Default|GetPlatform_Start_01_Cue) 0.0)
                      (Utilities|FlowControl|Sequence
                        (:then_0
                          (Utilities|FlowControl|Delay 5.0)
                          (Audio|Components|Audio|Play (Variables|Default|GetElevatorWarning_01_Cue) 0.0))
                        (:then_1
                          (Audio|Components|Audio|Play (Variables|Default|GetElevatorTone_01) 0.0 :!label _label))))
                    (:then_1
                      (switch Utilities|FlowControl|Switch|SwitchonETimelineDirection _direction
                        (:Forward
                          (CallFunction|PlatformReverese))
                        (:Backward
                          (CallFunction|PlatformForward)))
                      (Audio|Components|Audio|Play (Variables|Default|GetMotorLoop_02_Cue) 0.0))))
                (:then_1
                  (Audio|Components|Audio|Play (Variables|Default|GetSteamStop_01_03_Cue) 0.0)
                  (Utilities|FlowControl|Sequence
                    (:then_0
                      (Audio|Components|Audio|Stop (Variables|Default|GetMotorLoop_02_Cue)))
                    (:then_1
                      (goto _label))))
                (:then_2
                  ;[1 1 1] Doors Movement
                  (bind _doortravel (Timeline|DoorsTimeline PlayFromStart) ; Float Translation Curve
                    (:Update
                      _)
                    (:Finished
                      _))
                  (Transformation|SetRelativeLocation (Variables|Default|GetSM_RailDoor_L) (Math|Vector|Lerp(Vector) "0, 0, 0" "0,-48.000000, 0" (* _doortravel -1.0)) false false)
                  (Transformation|SetRelativeLocation (Variables|Default|GetSM_RailDoor_R) (Math|Vector|MakeVector (.X (Math|Vector|BreakVector (Math|Vector|Lerp(Vector) "0, 0, 0" "0,-48.000000, 0" (* _doortravel -1.0)))) (* (.Y (Math|Vector|BreakVector (Math|Vector|Lerp(Vector) "0, 0, 0" "0,-48.000000, 0" (* _doortravel -1.0)))) -1.0) (.Z (Math|Vector|BreakVector (Math|Vector|Lerp(Vector) "0, 0, 0" "0,-48.000000, 0" (* _doortravel -1.0))))) false false))))))
        (:then_1
          (bind _platform_rotation (Timeline|Platform%20Rotation%20Timeline Play) ; Float Rotation Curve
            (:Update
              (Transformation|SetRelativeRotation (Variables|Default|GetPlatform) (Math|Rotator|MakeRotator (.X (Math|Vector|BreakVector (Math|Vector|Lerp(Vector) "0, 0, 0" (Variables|PlatformControls|GetEndRotation) _platform_rotation))) (.Y (Math|Vector|BreakVector (Math|Vector|Lerp(Vector) "0, 0, 0" (Variables|PlatformControls|GetEndRotation) _platform_rotation))) (.Z (Math|Vector|BreakVector (Math|Vector|Lerp(Vector) "0, 0, 0" (Variables|PlatformControls|GetEndRotation) _platform_rotation)))) false false)))))
      (else
        (Utilities|FlowControl|Sequence
          (:then_0
            (Timeline|Platform%20Travel%20Timeline Reverse))
          (:then_1
            (Timeline|Platform%20Rotation%20Timeline Reverse)))))))

(event OnComponentBeginOverlap(DoorSafetyCollider)
  (params (OverlappedComponent :type Primitive%20Component%20Object%20Reference) (OtherActor :type Actor%20Object%20Reference) (OtherComp :type Primitive%20Component%20Object%20Reference) (OtherBodyIndex :type Integer) (bFromSweep :type Boolean) (SweepResult :type Hit%20Result%20Structure%20%28by%20ref%29))
  ;[1 1 1] Doors Movement
  ;;[1 1 1] Doors Safety Collision Open and Delayed Re-Close
  (Utilities|Casting|CastToBP_Char_Master OtherActor)
  (if (Components|Activation|IsActive (Variables|Default|GetDoorsTimeline))
    (Utilities|FlowControl|Sequence
      (:then_0
        (bind _doortravel (Timeline|DoorsTimeline Play) ; Float Translation Curve
          (:Update
            _)
          (:Finished
            _))
        (Transformation|SetRelativeLocation (Variables|Default|GetSM_RailDoor_L) (Math|Vector|Lerp(Vector) "0, 0, 0" "0,-48.000000, 0" (* _doortravel -1.0)) false false)
        (Transformation|SetRelativeLocation (Variables|Default|GetSM_RailDoor_R) (Math|Vector|MakeVector (.X (Math|Vector|BreakVector (Math|Vector|Lerp(Vector) "0, 0, 0" "0,-48.000000, 0" (* _doortravel -1.0)))) (* (.Y (Math|Vector|BreakVector (Math|Vector|Lerp(Vector) "0, 0, 0" "0,-48.000000, 0" (* _doortravel -1.0)))) -1.0) (.Z (Math|Vector|BreakVector (Math|Vector|Lerp(Vector) "0, 0, 0" "0,-48.000000, 0" (* _doortravel -1.0))))) false false))
      (:then_1
        (Utilities|FlowControl|Delay 2.0)
        (Timeline|DoorsTimeline ReverseFromEnd)))))

(event Custom|PlatformForward
  ;[1 1 1] Sets End Location and Rotation- Stop Delay- Reversing
  ;;[1 1 1] Reverses Direction if collision occurs with Actor
  (Utilities|FlowControl|Sequence
    (:then_0
      (bind (_direction _platform_travel) (Timeline|Platform%20Travel%20Timeline PlayFromStart) ; Float Translation Curve
        (:Update
          (Utilities|FlowControl|Sequence
            (:then_1
              (Transformation|SetRelativeLocation (Variables|Default|GetPlatform) (Math|Vector|Lerp(Vector) "0, 0, 0" (Variables|PlatformControls|GetEndLocation) _platform_travel) false false))))
        (:Finished
          (Utilities|FlowControl|Sequence
            (:then_0
              (Utilities|FlowControl|Delay (Variables|PlatformControls|GetStopDelay))
              (Utilities|FlowControl|Sequence
                (:then_0
                  ;[1 1 1] Start/Play/Stop Audio
                  (Audio|Components|Audio|Play (Variables|Default|GetPlatform_Start_01_Cue) 0.0)
                  (Utilities|FlowControl|Sequence
                    (:then_0
                      (Utilities|FlowControl|Delay 5.0)
                      (Audio|Components|Audio|Play (Variables|Default|GetElevatorWarning_01_Cue) 0.0))
                    (:then_1
                      (Audio|Components|Audio|Play (Variables|Default|GetElevatorTone_01) 0.0 :!label _label))))
                (:then_1
                  (switch Utilities|FlowControl|Switch|SwitchonETimelineDirection _direction
                    (:Forward
                      (CallFunction|PlatformReverese))
                    (:Backward
                      (CallFunction|PlatformForward)))
                  (Audio|Components|Audio|Play (Variables|Default|GetMotorLoop_02_Cue) 0.0))))
            (:then_1
              (Audio|Components|Audio|Play (Variables|Default|GetSteamStop_01_03_Cue) 0.0)
              (Utilities|FlowControl|Sequence
                (:then_0
                  (Audio|Components|Audio|Stop (Variables|Default|GetMotorLoop_02_Cue)))
                (:then_1
                  (goto _label))))
            (:then_2
              ;[1 1 1] Doors Movement
              (bind _doortravel (Timeline|DoorsTimeline PlayFromStart) ; Float Translation Curve
                (:Update
                  _)
                (:Finished
                  _))
              (Transformation|SetRelativeLocation (Variables|Default|GetSM_RailDoor_L) (Math|Vector|Lerp(Vector) "0, 0, 0" "0,-48.000000, 0" (* _doortravel -1.0)) false false)
              (Transformation|SetRelativeLocation (Variables|Default|GetSM_RailDoor_R) (Math|Vector|MakeVector (.X (Math|Vector|BreakVector (Math|Vector|Lerp(Vector) "0, 0, 0" "0,-48.000000, 0" (* _doortravel -1.0)))) (* (.Y (Math|Vector|BreakVector (Math|Vector|Lerp(Vector) "0, 0, 0" "0,-48.000000, 0" (* _doortravel -1.0)))) -1.0) (.Z (Math|Vector|BreakVector (Math|Vector|Lerp(Vector) "0, 0, 0" "0,-48.000000, 0" (* _doortravel -1.0))))) false false))))))
    (:then_1
      (bind _platform_rotation (Timeline|Platform%20Rotation%20Timeline PlayFromStart) ; Float Rotation Curve
        (:Update
          (Transformation|SetRelativeRotation (Variables|Default|GetPlatform) (Math|Rotator|MakeRotator (.X (Math|Vector|BreakVector (Math|Vector|Lerp(Vector) "0, 0, 0" (Variables|PlatformControls|GetEndRotation) _platform_rotation))) (.Y (Math|Vector|BreakVector (Math|Vector|Lerp(Vector) "0, 0, 0" (Variables|PlatformControls|GetEndRotation) _platform_rotation))) (.Z (Math|Vector|BreakVector (Math|Vector|Lerp(Vector) "0, 0, 0" (Variables|PlatformControls|GetEndRotation) _platform_rotation)))) false false))))
    (:then_2
      (Timeline|DoorsTimeline ReverseFromEnd))))

(event Custom|PlatformReverese
  ;[1 1 1] Sets End Location and Rotation- Stop Delay- Reversing
  ;;[1 1 1] Reverses Direction if collision occurs with Actor
  (Utilities|FlowControl|Sequence
    (:then_0
      (bind (_direction _platform_travel) (Timeline|Platform%20Travel%20Timeline ReverseFromEnd) ; Float Translation Curve
        (:Update
          (Utilities|FlowControl|Sequence
            (:then_1
              (Transformation|SetRelativeLocation (Variables|Default|GetPlatform) (Math|Vector|Lerp(Vector) "0, 0, 0" (Variables|PlatformControls|GetEndLocation) _platform_travel) false false))))
        (:Finished
          (Utilities|FlowControl|Sequence
            (:then_0
              (Utilities|FlowControl|Delay (Variables|PlatformControls|GetStopDelay))
              (Utilities|FlowControl|Sequence
                (:then_0
                  ;[1 1 1] Start/Play/Stop Audio
                  (Audio|Components|Audio|Play (Variables|Default|GetPlatform_Start_01_Cue) 0.0)
                  (Utilities|FlowControl|Sequence
                    (:then_0
                      (Utilities|FlowControl|Delay 5.0)
                      (Audio|Components|Audio|Play (Variables|Default|GetElevatorWarning_01_Cue) 0.0))
                    (:then_1
                      (Audio|Components|Audio|Play (Variables|Default|GetElevatorTone_01) 0.0 :!label _label))))
                (:then_1
                  (switch Utilities|FlowControl|Switch|SwitchonETimelineDirection _direction
                    (:Forward
                      (CallFunction|PlatformReverese))
                    (:Backward
                      (CallFunction|PlatformForward)))
                  (Audio|Components|Audio|Play (Variables|Default|GetMotorLoop_02_Cue) 0.0))))
            (:then_1
              (Audio|Components|Audio|Play (Variables|Default|GetSteamStop_01_03_Cue) 0.0)
              (Utilities|FlowControl|Sequence
                (:then_0
                  (Audio|Components|Audio|Stop (Variables|Default|GetMotorLoop_02_Cue)))
                (:then_1
                  (goto _label))))
            (:then_2
              ;[1 1 1] Doors Movement
              (bind _doortravel (Timeline|DoorsTimeline PlayFromStart) ; Float Translation Curve
                (:Update
                  _)
                (:Finished
                  _))
              (Transformation|SetRelativeLocation (Variables|Default|GetSM_RailDoor_L) (Math|Vector|Lerp(Vector) "0, 0, 0" "0,-48.000000, 0" (* _doortravel -1.0)) false false)
              (Transformation|SetRelativeLocation (Variables|Default|GetSM_RailDoor_R) (Math|Vector|MakeVector (.X (Math|Vector|BreakVector (Math|Vector|Lerp(Vector) "0, 0, 0" "0,-48.000000, 0" (* _doortravel -1.0)))) (* (.Y (Math|Vector|BreakVector (Math|Vector|Lerp(Vector) "0, 0, 0" "0,-48.000000, 0" (* _doortravel -1.0)))) -1.0) (.Z (Math|Vector|BreakVector (Math|Vector|Lerp(Vector) "0, 0, 0" "0,-48.000000, 0" (* _doortravel -1.0))))) false false))))))
    (:then_1
      (bind _platform_rotation (Timeline|Platform%20Rotation%20Timeline ReverseFromEnd) ; Float Rotation Curve
        (:Update
          (Transformation|SetRelativeRotation (Variables|Default|GetPlatform) (Math|Rotator|MakeRotator (.X (Math|Vector|BreakVector (Math|Vector|Lerp(Vector) "0, 0, 0" (Variables|PlatformControls|GetEndRotation) _platform_rotation))) (.Y (Math|Vector|BreakVector (Math|Vector|Lerp(Vector) "0, 0, 0" (Variables|PlatformControls|GetEndRotation) _platform_rotation))) (.Z (Math|Vector|BreakVector (Math|Vector|Lerp(Vector) "0, 0, 0" (Variables|PlatformControls|GetEndRotation) _platform_rotation)))) false false))))
    (:then_2
      (Timeline|DoorsTimeline ReverseFromEnd))))

(event EventBeginPlay
  (bind _traveltimeinseconds (Variables|PlatformControls|GetTravelTimeInSeconds))
  (bind _returnvalue (/ 1.0 _traveltimeinseconds))
  ;[1 1 1] Sets Travel/Rotation/Door Speed - Sets Preview Off - Starts Initial Sounds/Movement
  (Components|Timeline|SetPlayRate (Variables|Default|GetPlatform%20Travel%20Timeline) _returnvalue)
  (Components|Timeline|SetPlayRate (Variables|Default|GetPlatform%20Rotation%20Timeline) _returnvalue)
  (Components|Timeline|SetPlayRate (Variables|Default|GetDoorsTimeline) (/ 1.0 1.0))
  (Variables|PlatformControls|SetEndLocationPreview true) ; Safety to Defeat Preview during Play
  ;[1 1 1] Doors Movement
  (bind _doortravel (Timeline|DoorsTimeline ReverseFromEnd) ; Float Translation Curve
    (:Update
      _)
    (:Finished
      _))
  (Transformation|SetRelativeLocation (Variables|Default|GetSM_RailDoor_L) (Math|Vector|Lerp(Vector) "0, 0, 0" "0,-48.000000, 0" (* _doortravel -1.0)) false false)
  (Transformation|SetRelativeLocation (Variables|Default|GetSM_RailDoor_R) (Math|Vector|MakeVector (.X (Math|Vector|BreakVector (Math|Vector|Lerp(Vector) "0, 0, 0" "0,-48.000000, 0" (* _doortravel -1.0)))) (* (.Y (Math|Vector|BreakVector (Math|Vector|Lerp(Vector) "0, 0, 0" "0,-48.000000, 0" (* _doortravel -1.0)))) -1.0) (.Z (Math|Vector|BreakVector (Math|Vector|Lerp(Vector) "0, 0, 0" "0,-48.000000, 0" (* _doortravel -1.0))))) false false))

(fn ConstructionScript
  (bind _endrotation (Variables|PlatformControls|GetEndRotation))
  (bind _endlocationpreview (Variables|PlatformControls|GetEndLocationPreview))
  (bind _endlocation (Variables|PlatformControls|GetEndLocation))
  (bind _midpointpreview (Variables|PlatformControls|GetMidPointPreview))
  (bind _returnvalue (/ _endrotation 2))
  (bind _returnvalue_2 (Math|Vector|SelectVector _returnvalue _endrotation _midpointpreview))
  (bind _returnvalue_3 (Math|Vector|SelectVector _returnvalue_2 "0, 0, 0" _endlocationpreview))
  (bind (_x _y _z) (Math|Vector|BreakVector _returnvalue_3))
  (Transformation|SetRelativeLocation (Variables|Default|GetPlatform) (Math|Vector|SelectVector (Math|Vector|SelectVector (/ _endlocation 2) _endlocation (Variables|PlatformControls|GetMidPointPreview)) "0, 0, 0" _endlocationpreview) false false)
  (Transformation|SetRelativeRotation (Variables|Default|GetPlatform) (Math|Rotator|MakeRotator _x _y _z) false false))