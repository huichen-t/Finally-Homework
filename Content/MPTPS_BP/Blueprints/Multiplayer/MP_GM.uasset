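; Multiplayer game mode for a two-team score match with players and AI bots.
; New logins get the character select UI, then a polling timer spawns ready players at random team BP_PlayerSpawn points and possesses them.
; Another timer refills each team's bots one at a time against alive counts reduced by ReduceBotsAlive.
; PlayerDead updates team scores on every PC_MP, and a periodic check calls Back on all controllers once a team reaches five.
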(event Custom|生成就绪玩家
  ;[1 1 1] 玩家加入时随机生成 (复制到各个客户端)
  (for _array_element (Variables|Default|Get%20All%20players)
    (bind _aspc_mp (Utilities|Casting|CastToPC_MP _array_element))
    (if (Variables|/Game/MPTPS_BP/Blueprints/Multiplayer/PC_MP.PC_MP_C|GetIsReadySpawn _aspc_mp)
      (if (Variables|/Game/MPTPS_BP/Blueprints/Multiplayer/PC_MP.PC_MP_C|GetInSelectCharacter _aspc_mp)
        (if (Variables|/Game/MPTPS_BP/Blueprints/Multiplayer/PC_MP.PC_MP_C|GetTeam _aspc_mp)
          (bind _returnvalue (Game|SpawnActorfromClass "/Game/MPTPS_BP/Blueprints/Player/BP_Char_Master.BP_Char_Master_C" (Transformation|GetActorTransform (.OutItem (Utilities|Array|Random (Variables|Default|GetSpawnPointsA)))) "AlwaysSpawn" 0 0))
          (Utilities|IsValid _returnvalue
            (:Is%20Valid
              (Networking|SwitchHasAuthority
                (:Authority
                  (Pawn|Possess _aspc_mp _returnvalue)
                  (Default|SetReadySpawn _aspc_mp false)
                  (Default|BeginControlCharacter _aspc_mp)))))
          (else
            (bind _returnvalue_2 (Game|SpawnActorfromClass "/Game/MPTPS_BP/Blueprints/Player/BP_Char_Master.BP_Char_Master_C" (Transformation|GetActorTransform (.OutItem (Utilities|Array|Random (Variables|Default|GetSpawnPointsB)))) "AlwaysSpawn" 0 0))
            (Utilities|IsValid _returnvalue_2
              (:Is%20Valid
                (Networking|SwitchHasAuthority
                  (:Authority
                    (Pawn|Possess _aspc_mp _returnvalue_2)
                    (Default|SetReadySpawn _aspc_mp false)
                    (Default|BeginControlCharacter _aspc_mp)))))))))))

(event Custom|PlayerDead
  (params (ScoreTeam :type Boolean))
  ;[1 1 1] 注释
  (if ScoreTeam
    (bind _output_get (Variables|Default|SetTeamAScore (+ (Variables|Default|GetTeamAScore) 1)))
    (else
      (bind _output_get_2 (Variables|Default|SetTeamBScore (+ (Variables|Default|GetTeamBScore) 1)))))
  (for _array_element (Variables|Default|Get%20All%20players)
    (bind _aspc_mp (Utilities|Casting|CastToPC_MP _array_element))
    (Variables|/Game/MPTPS_BP/Blueprints/Multiplayer/PC_MP.PC_MP_C|SetTeamAScore _aspc_mp _output_get)
    (Variables|/Game/MPTPS_BP/Blueprints/Multiplayer/PC_MP.PC_MP_C|SetTeamBScore _aspc_mp _output_get_2)))

(event Custom|Check%20Win
  (if (>= (Variables|Default|GetTeamAScore) 5)
    (CallFunction|TeamWin true)
    (elif (>= (Variables|Default|GetTeamBScore) 5)
      (CallFunction|TeamWin false))))

(event Custom|TeamWin
  (params (Team :type Boolean))
  (for _array_element (Variables|Default|Get%20All%20players)
    (bind _aspc_mp (Utilities|Casting|CastToPC_MP _array_element))
    (Default|Back _aspc_mp Team)))

(event Custom|SpawnBots
  ;[0.1808 0.4349 1] Bots
  ;;[1 1 1] Spawn Bots
  (Utilities|FlowControl|Sequence
    (:then_0
      (if (> (- (Variables|Default|GetTeamABots) (Variables|Default|GetTeamABotsAlive)) 0)
        (bind _returnvalue (Game|SpawnActorfromClass "/Game/MPTPS_BP/Blueprints/Player/BP_AI_Pawn.BP_AI_Pawn_C" (Math|Conversions|ToTransform(Vector) (Transformation|GetActorLocation (.OutItem (Utilities|Array|Random (Variables|Default|GetSpawnPointsA))))) "Undefined" 0 0))
        (Variables|/Game/MPTPS_BP/Blueprints/Player/BP_Char_Master.BP_Char_Master_C|SetTeam _returnvalue true)
        (Variables|Default|SetTeamABotsAlive (+ (Variables|Default|GetTeamABotsAlive) 1))
        (Development|PrintString (Utilities|String|Append "现在A：" (Utilities|String|ToString(Integer) (Variables|Default|GetTeamABotsAlive))))))
    (:then_1
      (if (> (- (Variables|Default|GetTeamBBots) (Variables|Default|GetTeamBBotsAlive)) 0)
        (bind _returnvalue_2 (Game|SpawnActorfromClass "/Game/MPTPS_BP/Blueprints/Player/BP_AI_Pawn.BP_AI_Pawn_C" (Math|Conversions|ToTransform(Vector) (Transformation|GetActorLocation (.OutItem (Utilities|Array|Random (Variables|Default|GetSpawnPointsB))))) "Undefined" 0 0))
        (Variables|/Game/MPTPS_BP/Blueprints/Player/BP_Char_Master.BP_Char_Master_C|SetTeam _returnvalue_2 false)
        (Variables|Default|SetTeamBBotsAlive (+ (Variables|Default|GetTeamBBotsAlive) 1))
        (Development|PrintString (Utilities|String|Append "现在B：" (Utilities|String|ToString(Integer) (Variables|Default|GetTeamBBotsAlive))))))))

(event Custom|ReduceBotsAlive
  (params (Team :type Boolean))
  ;[0.1808 0.4349 1] Bots
  ;;[1 1 1] ReduceBotsAlive
  (if Team
    (bind _output_get (Variables|Default|SetTeamABotsAlive (- (Variables|Default|GetTeamABotsAlive) 1)))
    (else
      (bind _output_get_2 (Variables|Default|SetTeamBBotsAlive (- (Variables|Default|GetTeamBBotsAlive) 1))))))

(event Custom|ShowSelectCharacterUI
  ;[1 1 1] Show Select Character UI
  (for _array_element (Variables|Default|Get%20All%20players)
    (bind _aspc_mp (Utilities|Casting|CastToPC_MP _array_element))
    (if (Utilities|Enum|Equal(Enum) (Variables|/Game/MPTPS_BP/Blueprints/Multiplayer/PC_MP.PC_MP_C|GetMyPlayerState _aspc_mp) "NewEnumerator0")
      (Default|LoadCharacterSelectUI _aspc_mp))))

(event EventPostLogin
  (params (NewPlayer :type Player%20Controller%20Object%20Reference))
  (Utilities|Array|Add (Variables|Default|Get%20All%20players) NewPlayer)
  ;[1 1 1] 登录
  (bind _aspc_mp (Utilities|Casting|CastToPC_MP NewPlayer))
  (Variables|/Game/MPTPS_BP/Blueprints/Multiplayer/PC_MP.PC_MP_C|SetInSelectCharacter _aspc_mp true)
  (Variables|/Game/MPTPS_BP/Blueprints/Multiplayer/PC_MP.PC_MP_C|SetMyPlayerState _aspc_mp "NewEnumerator0")
  (CallFunction|ShowSelectCharacterUI))

(event EventBeginPlay
  ;[1 1 1] 玩家加入时随机生成 (复制到各个客户端)
  (Utilities|FlowControl|Sequence
    (:then_0
      (Utilities|Time|SetTimerbyEvent (delegate Custom|生成就绪玩家) 0.2 true)
      (bind _outactors (Actor|GetAllActorsOfClass "/Game/FPS/Blueprints/Misc/PlayerSpawn/BP_PlayerSpawn.BP_PlayerSpawn_C"))
      (bind _output_get (Variables|Default|SetSpawnPoints _outactors))
      (for _array_element _output_get
        (bind _asbp_player_spawn (Utilities|Casting|CastToBP_PlayerSpawn _array_element))
        (if (Variables|/Game/FPS/Blueprints/Misc/PlayerSpawn/BP_PlayerSpawn.BP_PlayerSpawn_C|GetbTeam _asbp_player_spawn)
          (Utilities|Array|Add (Variables|Default|GetSpawnPointsA) _asbp_player_spawn)
          (else
            (Utilities|Array|Add (Variables|Default|GetSpawnPointsB) _asbp_player_spawn)))))
    (:then_1
      (Variables|Default|SetTeamABots 4)
      (Variables|Default|SetTeamBBots 4)
      (Variables|Default|SetTeamABotsAlive 0)
      (Variables|Default|SetTeamBBotsAlive 0))
    (:then_2
      (Utilities|Time|SetTimerbyEvent (delegate Custom|SpawnBots) 6.0 true))
    (:then_3
      (Utilities|Time|SetTimerbyEvent (delegate Custom|Check%20Win) 1.0 true))))

(fn ConstructionScript
  (bind _outactors (Actor|GetAllActorsOfClass "/Script/Engine.PlayerStart"))
  (Variables|Default|SetSpawnPoints _outactors))