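; Multiplayer player controller that manages a player's team, character selection, main HUD and win-screen widgets, switching input mode and cursor for each.
; BeginControlCharacter clears widgets, sets game-only input and copies the stored team onto the possessed BP_Char_Master.
; CharacterDead reports the death to MP_GM, then after a delay sets the ready-to-spawn flag from the character's dead state.
; N, M and L keys directly trigger game mode win and death calls, apparently for testing.
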(event Custom|SetTeam
  (params (bTeam :type Boolean))
  ;[1 1 1] 设置队伍
  (Variables|Default|SetTeam bTeam))

(event Custom|SetReadySpawn
  (params (IsReadySpawn :type Boolean))
  ;[1 1 1] 设置队伍
  (Variables|Default|SetIsReadySpawn IsReadySpawn))

(event Custom|ClearWidgets
  ;[1 1 1] 清除所有控件
  (Viewport|RemoveAllWidgets))

(event Custom|BeginControlCharacter
  (bind _returnvalue (Game|Player|GetPlayerPawn 0))
  ;[1 1 1] 控制人物
  (CallFunction|ClearWidgets)
  (Variables|Default|SetMyPlayerState "NewEnumerator2")
  (Input|SetInputModeGameOnly self)
  (Variables|Default|SetbShowMouseCursor false)
  (Utilities|IsValid (Variables|Default|GetMainUI)
    (:Is%20Valid
      _)
    (:Is%20Not%20Valid
      (bind _returnvalue_2 (UserInterface|CreateWidget "/Game/MPTPS_BP/Blueprints/UI/W_Main.W_Main_C" self))
      (bind _output_get (Variables|Default|SetMainUI _returnvalue_2))))
  (UserInterface|Viewport|AddtoViewport _output_get 0)
  (Utilities|IsValid _returnvalue
    (:Is%20Valid
      (bind _asbp_char_master (Utilities|Casting|CastToBP_Char_Master _returnvalue))
      (Variables|/Game/MPTPS_BP/Blueprints/Player/BP_Char_Master.BP_Char_Master_C|SetTeam _asbp_char_master (Variables|Default|GetTeam)))))

(event Custom|Back
  (params (WinTeam :type Boolean))
  (bind _self self)
  (Utilities|IsValid (Variables|Default|GetWinGame)
    (:Is%20Valid
      _)
    (:Is%20Not%20Valid
      (bind _returnvalue (UserInterface|CreateWidget "/Game/MPTPS_BP/Blueprints/Multiplayer/Widgets/W_WinGame.W_WinGame_C" self))
      (Variables|Default|SetWinGame _returnvalue)))
  (UserInterface|Viewport|AddtoViewport (Variables|Default|GetWinGame) 0)
  (Input|SetInputModeUIOnly _self (Variables|Default|GetWinGame) "DoNotLock")
  (Variables|Default|SetbShowMouseCursor _self true)
  (Variables|/Game/MPTPS_BP/Blueprints/Multiplayer/Widgets/W_WinGame.W_WinGame_C|SetWinTeam (Variables|Default|GetWinGame) WinTeam))

(event Custom|CharacterDead
  (bind _asmp_gm (Utilities|Casting|CastToMP_GM (Game|GetGameMode)))
  (Default|PlayerDead _asmp_gm (Variables|Default|GetTeam))
  (Utilities|FlowControl|Delay 2.0)
  (bind _asbp_char_master (Utilities|Casting|CastToBP_Char_Master (Game|Player|GetPlayerPawn 0)))
  (CallFunction|SetReadySpawn (Variables|/Game/MPTPS_BP/Blueprints/Player/BP_Char_Master.BP_Char_Master_C|GetIsDead? _asbp_char_master)))

(event Custom|LoadCharacterSelectUI
  (bind _self self)
  ;[1 1 1] 人物选择UI
  (Utilities|IsValid (Variables|Default|GetCharacterSelection)
    (:Is%20Valid
      _)
    (:Is%20Not%20Valid
      (bind _returnvalue (UserInterface|CreateWidget "/Game/MPTPS_BP/Blueprints/Multiplayer/Widgets/W_CharacterSelection.W_CharacterSelection_C" self))
      (Variables|Default|SetCharacterSelection _returnvalue)))
  (UserInterface|Viewport|AddtoViewport (Variables|Default|GetCharacterSelection) 0)
  (Input|SetInputModeUIOnly _self (Variables|Default|GetCharacterSelection) "DoNotLock")
  (Variables|Default|SetbShowMouseCursor _self true))

(event Input|KeyboardEvents|L
  (params (Key :type Key%20Structure :default "None"))
  (:Pressed
    (bind _asmp_gm (Utilities|Casting|CastToMP_GM (Game|GetGameMode)))
    (Default|PlayerDead _asmp_gm false)))

(event Input|KeyboardEvents|N
  (params (Key :type Key%20Structure :default "None"))
  (:Pressed
    (bind _asmp_gm (Utilities|Casting|CastToMP_GM (Game|GetGameMode)))
    (Default|TeamWin _asmp_gm false)))

(event Input|KeyboardEvents|M
  (params (Key :type Key%20Structure :default "None"))
  (:Pressed
    (bind _asmp_gm (Utilities|Casting|CastToMP_GM (Game|GetGameMode)))
    (Default|PlayerDead _asmp_gm true)))

(fn ConstructionScript)