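; MotusMan demo character that loops an animation and sound, takes damage, dies and respawns in place.
; AnyDamage clamps health and, at zero, calls a multicast kill event so every client sees the death.
; A DoOnce, reset on Tick while alive, runs the death sequence: sound, animation, timed hide with collision off.
; After RespawnRate, it restores visibility, collision, loops and full health.
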(event Custom|Multicast_KillMotusMan
  ;[1 1 1] Multicast Kill MotusMan Event This Is Everything That Is Done To Replicate The Death For Everyone To View
  (Variables|Default|SetIsMotusManDead? true)
  (Utilities|FlowControl|DoOnce false
    (:Completed
      (Audio|Components|Audio|FadeOut (Variables|Default|GetAudioLoop) 0.1 0.0 :!class /Script/Engine.AudioComponent)
      (Audio|SpawnSoundAttached (Variables|Default|GetDeathSound) (Variables|Default|GetSkeletalMesh) "Neck1")
      (Components|Animation|PlayAnimation (Variables|Default|GetSkeletalMesh) (Variables|Default|GetDeathAnimation) false)
      (Utilities|FlowControl|Delay 8.7)
      (Collision|SetCollisionEnabled (Variables|Default|GetSkeletalMesh) "NoCollision")
      (Rendering|SetActorHiddenInGame true)
      (Utilities|FlowControl|Delay (Variables|Default|GetRespawnRate))
      (Collision|SetCollisionEnabled (Variables|Default|GetSkeletalMesh) "QueryAndPhysics")
      (Rendering|SetActorHiddenInGame false)
      (Audio|Components|Audio|FadeIn (Variables|Default|GetAudioLoop) 0.1 1.0 0.0 :!class /Script/Engine.AudioComponent)
      (Components|Animation|PlayAnimation (Variables|Default|GetSkeletalMesh) (Variables|Default|GetDemoAnimation) true)
      (Variables|Default|SetIsMotusManDead? false)
      (Variables|Default|SetCurrentHealth (Variables|Default|GetMaxHealth)))))

(event EventBeginPlay
  ;[0.9913 1 0] Event Begin Play Set MotusMans Health Start The Loop Animation & Sound Loop
  (Variables|Default|SetCurrentHealth (Variables|Default|GetMaxHealth))
  (Components|Animation|PlayAnimation (Variables|Default|GetSkeletalMesh) (Variables|Default|GetDemoAnimation) true)
  (Audio|Components|Audio|FadeIn (Variables|Default|GetAudioLoop) 0.1 1.0 0.0 :!class /Script/Engine.AudioComponent))

(event Game|Damage|EventAnyDamage
  (params (Damage :type Float%20%28single-precision%29) (DamageType :type Damage%20Type%20Object%20Reference) (InstigatedBy :type Controller%20Object%20Reference) (DamageCauser :type Actor%20Object%20Reference))
  ;[1 0 0] Apply Damage & Kill Motun Man Calls Multicast Event For Replication
  (Variables|Default|SetCurrentHealth (Math|Integer|Clamp(Integer) (Math|Float|Truncate (- (Math|Conversions|ToFloat(Integer) (Variables|Default|GetCurrentHealth)) Damage)) 0 (Variables|Default|GetMaxHealth)))
  (if (== (Variables|Default|GetCurrentHealth) 0)
    (CallFunction|MulticastKillMotusMan)))

(event EventTick
  (params (DeltaSeconds :type Float%20%28single-precision%29))
  ;[1 0.4923 0] Event Tick This Monitors If Motus Man Is Dead Or Not To Reset DoOnce
  (if (not (Variables|Default|GetIsMotusManDead?))
    ;[1 1 1] Multicast Kill MotusMan Event This Is Everything That Is Done To Replicate The Death For Everyone To View
    (Utilities|FlowControl|DoOnce false) ; enters at Reset
  ))

(fn ConstructionScript)