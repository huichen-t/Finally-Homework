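; BP_Wep_Station is a weapon station actor where a player can swap weapons while standing in its overlap area.
; Begin and end overlap cast to BP_Char_Master and its PC_MP controller, then call client events that enable or disable the station's input for that controller.
; Number keys 1–5 call matching ServerSwapToWeapon functions on the character cast from the begin overlap.
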(event Custom|Client_OnStationEnter
  (params (PlayerController :type PC%20MP%20Object%20Reference))
  (Input|EnableInput PlayerController))

(event Custom|Client_OnStationExit
  (params (PlayerController :type PC%20MP%20Object%20Reference))
  (Input|DisableInput PlayerController))

(event Collision|EventActorBeginOverlap
  (params (OtherActor :type Actor%20Object%20Reference))
  (bind _asbp_char_master (Utilities|Casting|CastToBP_Char_Master OtherActor))
  (bind _aspc_mp (Utilities|Casting|CastToPC_MP (Pawn|GetController _asbp_char_master)))
  (CallFunction|ClientonStationEnter _aspc_mp))

(event Collision|EventActorEndOverlap
  (params (OtherActor :type Actor%20Object%20Reference))
  (bind _asbp_char_master (Utilities|Casting|CastToBP_Char_Master OtherActor))
  (bind _aspc_mp (Utilities|Casting|CastToPC_MP (Pawn|GetController _asbp_char_master)))
  (CallFunction|ClientonStationExit _aspc_mp))

(event Input|KeyboardEvents|1
  (params (Key :type Key%20Structure))
  (:Pressed
    (Default|ServerSwaptoWeapon0 (stale Collision|EventActorBeginOverlap _asbp_char_master))))

(event Input|KeyboardEvents|2
  (params (Key :type Key%20Structure))
  (:Pressed
    (Default|ServerSwaptoWeapon1 (stale Collision|EventActorBeginOverlap _asbp_char_master))))

(event Input|KeyboardEvents|3
  (params (Key :type Key%20Structure))
  (:Pressed
    (Default|ServerSwaptoWeapon2 (stale Collision|EventActorBeginOverlap _asbp_char_master))))

(event Input|KeyboardEvents|4
  (params (Key :type Key%20Structure))
  (:Pressed
    (Default|ServerSwaptoWeapon3 (stale Collision|EventActorBeginOverlap _asbp_char_master))))

(event Input|KeyboardEvents|5
  (params (Key :type Key%20Structure))
  (:Pressed
    (Default|ServerSwaptoWeapon4 (stale Collision|EventActorBeginOverlap _asbp_char_master))))

(fn ConstructionScript)