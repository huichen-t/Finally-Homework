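; BP_AI_Pawn is a pawn Blueprint for AI bots that reports the bot's death to its AI controller.
; On_Dead_bot casts the pawn's controller to AI_BOT_Controller and calls Dead with the pawn's Team, doing nothing if the cast fails.
; The event graph holds only disabled default events, the construction script just calls the parent, and one extra function is an empty placeholder.
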(event EventBeginPlay
  (|CallParentFunction) ; 此节点被禁用，将不会被调用。\n从引脚连出引线来编译功能。
)

(event Collision|EventActorBeginOverlap
  (params (OtherActor :type Actor%20Object%20Reference)))

(event EventTick
  (params (DeltaSeconds :type Float%20%28single-precision%29))
  (|CallParentFunction DeltaSeconds) ; 此节点被禁用，将不会被调用。\n从引脚连出引线来编译功能。
)

(fn ConstructionScript
  (|CallParentFunction))

(fn 新函数0)

(fn OnDeadBot
  (bind _asai_bot_controller (Utilities|Casting|CastToAI_BOT_Controller (AI|GetAIController self)))
  (Default|Dead _asai_bot_controller (Variables|Default|GetTeam)))