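; Master multiplayer weapon Blueprint supporting single, auto, burst, multi and stream fire, plus ammo, reload and scope zoom.
; Client-side fire-mode macros pace sphere traces and send hits to the server.
; The server applies hitscan damage (headshot or radial) or spawns a projectile, updates ammo and cooldown, then multicasts per-mode effects.
; Gate and DoOnce macros control repeat fire, looping audio and the stream beam; scope uses a Timeline for FOV and HUD.
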(event Custom|Client_OnWeaponFire
  ;[1 1 1] 开火模式
  (switch Utilities|FlowControl|Switch|SwitchonE_WeaponFiringModes (Variables|Default|GetFiringMode)
    (:NewEnumerator1
      ;[1 1 1] Weapon Firing Modes
      (Utilities|SingleFireMode
        (:Out
          _)))
    (:NewEnumerator2
      (Utilities|AutoFireMode
        (:Out
          _)))
    (:NewEnumerator3
      (Utilities|BurstFireMode
        (:Out
          _)))
    (:NewEnumerator4
      (Utilities|MultiFireMode
        (:Out
          _)))
    (:NewEnumerator5
      (Utilities|StreamFireMode
        (:Out
          _))))
  ;[1 1 1] SphereTrace And Stop Weapon Fire When Ammo Is 0  Call Server Shoot Info
  (bind (_hitresult _hit) (CallFunction|SphereTrace))
  (if (not (== (Variables|DoNotSetVariables|GetCurrentAmmoInClip) 0))
    (CallFunction|ServerShootInfo _hitresult _hit)
    (else
      (Default|ServerStopFireWeapon (.AsBP%20Char%20Master (Utilities|Casting|CastToBP_Char_Master (Game|Player|GetPlayerPawn 0)))))))

(event Custom|Bandplayer
  (params (controller :type BP%20Char%20Master%20Object%20Reference))
  (Variables|Default|Setcontroller controller))

(event Custom|Multicast_SingleFireWeaponFX
  (params (HitResult :type Hit%20Result%20Structure) (Hit :type Boolean))
  ;[1 1 1] Single Fire Weapon FX
  (CallFunction|SingleFireWeaponFX HitResult Hit))

(event Custom|Server_ShootInfo
  (params (HitResult :type Hit%20Result%20Structure) (Hit :type Boolean))
  ;[1 1 1] Set Weapon Cooldown And Calculate Damage And Spawn Projectile In Shoot Info
  (Variables|DoNotSetVariables|SetIsWeaponCooldownActive? true)
  (bind (_hitresultout _hitout) (CallFunction|ShootInfo HitResult Hit))
  ;[1 1 1] Firing Mode Selection Enum
  (switch Utilities|FlowControl|Switch|SwitchonE_WeaponFiringModes (Variables|Default|GetFiringMode)
    (:NewEnumerator1
      ;[1 1 1] Call Weapon Multicast Effects
      (CallFunction|MulticastSingleFireWeaponFX _hitresultout _hitout))
    (:NewEnumerator2
      (Variables|DoNotSetVariables|SetIsAutoFireWeapon? true)
      (CallFunction|MulticastAutoFireWeaponFX _hitresultout _hitout))
    (:NewEnumerator3
      (CallFunction|MulticastBurstFireWeaponFX _hitresultout _hitout))
    (:NewEnumerator4
      (CallFunction|MulticastMultiFireWeaponFX _hitresultout _hitout)
      (Utilities|FlowControl|DoOnce false
        (:Completed
          _)))
    (:NewEnumerator5
      (Variables|DoNotSetVariables|SetIsAutoFireWeapon? true)
      (CallFunction|MulticastStreamFireWeaponFX _hitresultout _hitout)))
  ;[1 1 1] Decrement Ammo And Set Weapon Cooldown
  (CallFunction|DecrementAmmo)
  (Utilities|FlowControl|Delay (Variables|Default|GetCooldown))
  (Variables|DoNotSetVariables|SetIsWeaponCooldownActive? false))

(event Custom|Multicast_MultiFireWeaponFX
  (params (HitResult :type Hit%20Result%20Structure) (Hit :type Boolean))
  ;[1 1 1] MutiFire Weapon FX
  (Utilities|FlowControl|Sequence
    (:then_0
      (CallFunction|MultiFireWeaponFX HitResult Hit))
    (:then_1
      ;;[1 1 1] This Is A Macro That Controls A DoOnce For The Playing Of The Firing Sound AnSpawning Of The Muzzle Flash
      (Utilities|MultiFireModeDoOnce))))

(event Custom|Multicast_BurstFireWeaponFX
  (params (HitResult :type Hit%20Result%20Structure) (Hit :type Boolean))
  ;[1 1 1] BurstFire Weapon FX
  (CallFunction|BurstFireWeaponFX HitResult Hit))

(event Custom|Multicast_AutoFireWeaponFX
  (params (HitResult :type Hit%20Result%20Structure) (Hit :type Boolean))
  ;[1 1 1] AutoFire Weapon FX
  (Utilities|FlowControl|Sequence
    (:then_0
      (CallFunction|AutoFireWeaponFX HitResult Hit))
    (:then_1
      ;;[1 1 1] This Is To Fade In & Out Sound If Weapon Is AutoFire Also Play Shot End Sound
      (Utilities|AutoFireSoundControl))))

(event Custom|Client_PlayDryFireSound
  ;[1 1 1] Client Play DryFire Sound (Not Replicated)
  (Audio|PlaySoundatLocation (Variables|Effects|GetDryFireSound) (Transformation|GetActorLocation) "0, 0, 0" 1.0 1.0 0.0 0 0 0))

(event Custom|Client_OffWeaponFire
  ;[0.9977 1 0] Client Off Weapon Fire Call Server Off Weapon Fire
  (Utilities|FlowControl|Sequence
    (:then_0
      (CallFunction|ServerOffWeaponFire))
    (:then_1
      ;[1 1 1] Weapon Firing Modes
      (Utilities|AutoFireMode) ; enters at CloseGate
    )
    (:then_2
      (Utilities|StreamFireMode) ; enters at CloseGate
    )))

(event Custom|Client_ActivateScope
  (bind _returnvalue (Game|Player|GetPlayerPawn 0))
  (bind _asbp_char_master (Utilities|Casting|CastToBP_Char_Master _returnvalue))
  ;[1 1 1] Scope Activate/Deactivate
  (Class|PrimitiveComponent|SetOwnerNoSee (Variables|/Script/Engine.Character|GetMesh _asbp_char_master) true :!pinned true) ; Sets Player Invisible when Scope is Activated
  (Class|PrimitiveComponent|SetOwnerNoSee (Variables|Default|GetWeaponMesh) true :!pinned true) ; Sets Weapon Invisible when Scope is Activated
  (bind (_direction _fieldofview _scopeopacity) (Timeline|ScopeTimeLine Play)
    (:Update
      (Variables|/Script/Engine.CameraComponent|SetFieldOfView (Variables|/Game/MPTPS_BP/Blueprints/Player/BP_Char_Master.BP_Char_Master_C|GetFollowCam _asbp_char_master) _fieldofview)
      (bind _asbp_my_hud (Utilities|Casting|CastToBP_MyHUD (HUD|GetHUD (Game|GetPlayerController 0))))
      (Variables|/Game/MPTPS_BP/Blueprints/UI/BP_MyHUD.BP_MyHUD_C|SetScopeOpacity _asbp_my_hud _scopeopacity))))

(event Custom|Server_OnWeaponReload
  ;[1 1 1] Reload Add Ammo
  (Utilities|FlowControl|Delay 1.1)
  (CallFunction|MulticastReloadSound)
  (CallFunction|ReloadAddAmmo))

(event Custom|Client_DeactivateScope
  (bind _returnvalue (Game|Player|GetPlayerPawn 0))
  (bind _asbp_char_master (Utilities|Casting|CastToBP_Char_Master _returnvalue))
  ;[1 1 1] Scope Activate/Deactivate
  (Class|PrimitiveComponent|SetOwnerNoSee (Variables|/Script/Engine.Character|GetMesh _asbp_char_master) false)
  (Class|PrimitiveComponent|SetOwnerNoSee (Variables|Default|GetWeaponMesh) false)
  (bind (_direction _fieldofview _scopeopacity) (Timeline|ScopeTimeLine Reverse)
    (:Update
      (Variables|/Script/Engine.CameraComponent|SetFieldOfView (Variables|/Game/MPTPS_BP/Blueprints/Player/BP_Char_Master.BP_Char_Master_C|GetFollowCam _asbp_char_master) _fieldofview)
      (bind _asbp_my_hud (Utilities|Casting|CastToBP_MyHUD (HUD|GetHUD (Game|GetPlayerController 0))))
      (Variables|/Game/MPTPS_BP/Blueprints/UI/BP_MyHUD.BP_MyHUD_C|SetScopeOpacity _asbp_my_hud _scopeopacity))))

(event Custom|Server_OffWeaponFire
  ;[1 0.8515 0] Server Off WeaponFire To Multicast Off Weapon Fire
  (Utilities|FlowControl|Sequence
    (:then_0
      (CallFunction|MulticastOffWeaponFire))
    (:then_1
      ;[1 1 1] Call Weapon Multicast Effects
      (Utilities|FlowControl|DoOnce false) ; enters at Reset
    )))

(event Custom|Multicast_StreamFireWeaponFX
  (params (HitResult :type Hit%20Result%20Structure) (Hit :type Boolean))
  ;[1 1 1] Stream Fire Weapon FX
  (Utilities|FlowControl|Sequence
    (:then_0
      (CallFunction|StreamFireWeaponFX HitResult Hit))
    (:then_1
      ;;[1 1 1] This Is To Fade In & Out Sound If Weapon Is AutoFire Also Play Shot End Sound
      (Utilities|AutoFireSoundControl))
    (:then_2
      ;;[1 1 1] This Is A Macro That Controls The Particle Beam For Beam Fire Weapons
      (Utilities|StreamFirePSControl Hit HitResult))))

(event Custom|Multicast_ReloadSound
  ;[1 1 1] Reload Add Ammo
  (Audio|SpawnSoundAttached (Variables|Effects|GetReloadSound) (Variables|Default|GetWeaponMesh) (Variables|Default|GetMuzzleSocketName) "0, 0, 0" "0, 0, 0" "KeepRelativeOffset" false 1.0 1.0 0.0 0 0))

(event Custom|Multicast_OffWeaponFire
  ;[1 0.9431 0] Multicast  Off Weapon Fire
  (Utilities|FlowControl|Sequence
    (:then_0
      ;[1 1 1] AutoFire Weapon FX
      (Utilities|FlowControl|Sequence
        (:then_0
          ;;[1 1 1] This Is To Fade In & Out Sound If Weapon Is AutoFire Also Play Shot End Sound
          (Utilities|AutoFireSoundControl) ; enters at ResetDoOnce
        )
        (:then_1
          (Utilities|AutoFireSoundControl) ; enters at FadeOutAudio
        )))
    (:then_1
      ;[1 1 1] MutiFire Weapon FX
      ;;[1 1 1] This Is A Macro That Controls A DoOnce For The Playing Of The Firing Sound AnSpawning Of The Muzzle Flash
      (Utilities|MultiFireModeDoOnce) ; enters at ResetDoOnce
    )
    (:then_2
      ;[1 1 1] Stream Fire Weapon FX
      (Utilities|FlowControl|Sequence
        (:then_0
          ;;[1 1 1] This Is To Fade In & Out Sound If Weapon Is AutoFire Also Play Shot End Sound
          (Utilities|AutoFireSoundControl) ; enters at ResetDoOnce
        )
        (:then_1
          (Utilities|AutoFireSoundControl) ; enters at FadeOutAudio
        )
        (:then_2
          ;;[1 1 1] This Is A Macro That Controls The Particle Beam For Beam Fire Weapons
          (Utilities|StreamFirePSControl (stale Custom|Multicast_StreamFireWeaponFX Hit) (stale Custom|Multicast_StreamFireWeaponFX HitResult)) ; enters at CloseGateDeactivateParticle
        )))))

(event EventBeginPlay
  ;[1 0.9886 0] Event Begin Play Server Set Weapon Ammo
  (Networking|SwitchHasAuthority
    (:Authority
      (Variables|DoNotSetVariables|SetCurrentMaxAmmo (Variables|Default|GetMaxAmmo))
      (Variables|DoNotSetVariables|SetCurrentAmmoInClip (Variables|Default|GetMaxAmmoClipSize)))))

(fn ConstructionScript)

(fn SphereTrace
  (bind _controller (Variables|Default|Getcontroller))
  (bind _spheretracestartlocation (Variables|/Game/MPTPS_BP/Blueprints/Player/BP_Char_Master.BP_Char_Master_C|GetSphereTraceStartLocation _controller))
  (bind _returnvalue (Transformation|GetWorldLocation _spheretracestartlocation))
  (bind (_outhit _returnvalue_2) (Collision|SphereTraceByChannel _returnvalue (Utilities|RandomWeaponSpread (+ _returnvalue (* (Math|Vector|GetForwardVector (Transformation|GetWorldRotation _spheretracestartlocation)) (Variables|Default|GetRange)))) (Variables|Default|GetSphereTraceRadius) "TraceTypeQuery1" false (Utilities|Array|MakeArray _controller) "None"))
  (return _outhit _returnvalue_2))

(fn ShootInfo
  (params (HitResult :type Hit%20Result%20Structure) (Hit :type Boolean%20%28by%20ref%29))
  (bind (_bblockinghit _binitialoverlap _time _distance _location _impactpoint _normal _impactnormal _physmat _hitactor _hitcomponent _hitbonename _hititem _elementindex _faceindex _tracestart _traceend) (Collision|BreakHitResult HitResult))
  (bind _returnvalue (Game|GetInstigatorController))
  (bind _self self)
  (bind _hitscanmaxdamage (Variables|HitscanWeaponConfig|GetHitScanMaxDamage))
  (bind _weaponmesh (Variables|Default|GetWeaponMesh))
  (bind _muzzlesocketname (Variables|Default|GetMuzzleSocketName))
  (bind _hitscanmindamage (Variables|HitscanWeaponConfig|GetHitScanMinDamage))
  (bind _returnvalue_2 (Transformation|GetSocketLocation _weaponmesh _muzzlesocketname))
  (bind _returnvalue_3 (Math|Random|RandomIntegerinRange _hitscanmindamage _hitscanmaxdamage))
  (bind _returnvalue_4 (Math|Conversions|ToFloat(Integer) _returnvalue_3))
  (Networking|SwitchHasAuthority
    (:Authority
      (if (Variables|HitscanWeaponConfig|GetIsHitScanWeapon?)
        (if Hit
          ;[1 1 1] Deal Damage If This Is A Hitscan Weapon
          (switch Utilities|FlowControl|Switch|SwitchonE_DamageTypes (Variables|HitscanWeaponConfig|GetHitScanDamageType)
            (:NewEnumerator0
              _)
            (:NewEnumerator1
              (switch name _hitbonename
                (:Default
                  (Game|Damage|ApplyDamage _hitactor _returnvalue_4 _returnvalue _self))
                (:Head
                  (Game|Damage|ApplyDamage _hitactor (Math|Conversions|ToFloat(Integer) (* _returnvalue_3 (Variables|HitscanWeaponConfig|GetHitScanCriticalMultiplier))) _returnvalue _self))))
            (:NewEnumerator2
              (Game|Damage|ApplyRadialDamage _returnvalue_4 _impactpoint (Variables|HitscanWeaponConfig|GetHitscanAreaOfEffect) 0 0 _self _returnvalue false "ECC_Visibility"))))
        (else
          ;[1 1 1] If Not A Hitscan Weapon Spawn A projectile Instead
          (Game|SpawnActorfromClass (Variables|Default|GetProjectile) (Math|Transform|MakeTransform _returnvalue_2 (Math|Rotator|FindLookatRotation _returnvalue_2 (Math|Vector|SelectVector _impactpoint _traceend Hit))) "AlwaysSpawn" (Components|GetOwner) (Game|GetInstigator)))))
    (:Remote
      _))
  (return HitResult Hit))

(fn ReloadAddAmmo
  (Networking|SwitchHasAuthority
    (:Authority
      (Variables|DoNotSetVariables|SetAmmoNeededForReload (- (Variables|Default|GetMaxAmmoClipSize) (Variables|DoNotSetVariables|GetCurrentAmmoInClip)))
      (if (<= (Variables|DoNotSetVariables|GetCurrentMaxAmmo) (Variables|DoNotSetVariables|GetAmmoNeededForReload))
        (Variables|DoNotSetVariables|SetCurrentAmmoInClip (+ (Variables|DoNotSetVariables|GetCurrentAmmoInClip) (Variables|DoNotSetVariables|GetCurrentMaxAmmo)))
        (Variables|DoNotSetVariables|SetCurrentMaxAmmo 0)
        (else
          (Variables|DoNotSetVariables|SetCurrentMaxAmmo (- (Variables|DoNotSetVariables|GetCurrentMaxAmmo) (Variables|DoNotSetVariables|GetAmmoNeededForReload)))
          (Variables|DoNotSetVariables|SetCurrentAmmoInClip (Variables|Default|GetMaxAmmoClipSize)))))))

(fn DecrementAmmo
  (Variables|DoNotSetVariables|SetCurrentAmmoInClip (Math|Integer|Clamp(Integer) (- (Variables|DoNotSetVariables|GetCurrentAmmoInClip) 1) 0 (Variables|Default|GetMaxAmmoClipSize))))

(fn SingleFireWeaponFX
  (params (HitResult :type Hit%20Result%20Structure) (Hit :type Boolean%20%28by%20ref%29))
  (bind (_bblockinghit _binitialoverlap _time _distance _location _impactpoint _normal _impactnormal _physmat) (Collision|BreakHitResult HitResult))
  (bind _muzzlesocketname (Variables|Default|GetMuzzleSocketName))
  ;[1 1 1] Play Firing Sound & Spawn Muzzle Flash (Sound Played Here Is For Not Auto Fire Weapons)
  (Audio|SpawnSoundAttached (Variables|Effects|GetSingleFireSound) (Variables|Default|GetWeaponMesh) _muzzlesocketname "0, 0, 0" "0, 0, 0" "KeepRelativeOffset" false 1.0 1.0 0.0 0 0)
  (Effects|SpawnEmitterAttached (Variables|Effects|GetMuzzleFlashPS) (Variables|Default|GetWeaponMesh) _muzzlesocketname)
  (if (Variables|HitscanWeaponConfig|GetIsHitScanWeapon?)
    (if Hit
      ;[1 1 1] Play Impact Particle & Sound Based On Pysical Material
      (Audio|PlaySoundatLocation (Utilities|Select :Index (Variables|/Script/PhysicsCore.PhysicalMaterial|GetSurfaceType _physmat) :SurfaceType_Default (Variables|HitscanWeaponConfig|GetHitscanDefaultImpactSound) :SurfaceType1 (Variables|HitscanWeaponConfig|GetHitscanCharacterImpactSound)) _impactpoint "0, 0, 0" 1.0 1.0 0.0 0 0 0)
      (Effects|SpawnEmitteratLocation (Utilities|Select :Index (Variables|/Script/PhysicsCore.PhysicalMaterial|GetSurfaceType _physmat) :SurfaceType_Default (Variables|HitscanWeaponConfig|GetHitscanDefaultImpactPS) :SurfaceType1 (Variables|HitscanWeaponConfig|GetHitscanCharacterImpactPS)) _impactpoint (Math|Conversions|RotationFromXVector _impactnormal)))))

(fn AutoFireWeaponFX
  (params (HitResult :type Hit%20Result%20Structure) (Hit :type Boolean%20%28by%20ref%29))
  (bind (_bblockinghit _binitialoverlap _time _distance _location _impactpoint _normal _impactnormal _physmat) (Collision|BreakHitResult HitResult))
  ;[1 1 1] Play Firing Sound & Spawn Muzzle Flash (Sound Played Here Is For Not Auto Fire Weapons)
  (Effects|SpawnEmitterAttached (Variables|Effects|GetMuzzleFlashPS) (Variables|Default|GetWeaponMesh) (Variables|Default|GetMuzzleSocketName))
  (if (Variables|HitscanWeaponConfig|GetIsHitScanWeapon?)
    (if Hit
      ;[1 1 1] Play Impact Particle & Sound Based On Pysical Material
      (Audio|PlaySoundatLocation (Utilities|Select :Index (Variables|/Script/PhysicsCore.PhysicalMaterial|GetSurfaceType _physmat) :SurfaceType_Default (Variables|HitscanWeaponConfig|GetHitscanDefaultImpactSound) :SurfaceType1 (Variables|HitscanWeaponConfig|GetHitscanCharacterImpactSound)) _impactpoint "0, 0, 0" 1.0 1.0 0.0 0 0 0)
      (Effects|SpawnEmitteratLocation (Utilities|Select :Index (Variables|/Script/PhysicsCore.PhysicalMaterial|GetSurfaceType _physmat) :SurfaceType_Default (Variables|HitscanWeaponConfig|GetHitscanDefaultImpactPS) :SurfaceType1 (Variables|HitscanWeaponConfig|GetHitscanCharacterImpactPS)) _impactpoint (Math|Conversions|RotationFromXVector _impactnormal)))))

(fn BurstFireWeaponFX
  (params (HitResult :type Hit%20Result%20Structure) (Hit :type Boolean%20%28by%20ref%29))
  (bind (_bblockinghit _binitialoverlap _time _distance _location _impactpoint _normal _impactnormal _physmat) (Collision|BreakHitResult HitResult))
  (bind _muzzlesocketname (Variables|Default|GetMuzzleSocketName))
  ;[1 1 1] Play Firing Sound & Spawn Muzzle Flash (Sound Played Here Is For Not Auto Fire Weapons)
  (Audio|SpawnSoundAttached (Variables|Effects|GetSingleFireSound) (Variables|Default|GetWeaponMesh) _muzzlesocketname "0, 0, 0" "0, 0, 0" "KeepRelativeOffset" false 1.0 1.0 0.0 0 0)
  (Effects|SpawnEmitterAttached (Variables|Effects|GetMuzzleFlashPS) (Variables|Default|GetWeaponMesh) _muzzlesocketname)
  (if (Variables|HitscanWeaponConfig|GetIsHitScanWeapon?)
    (if Hit
      ;[1 1 1] Play Impact Particle & Sound Based On Pysical Material
      (Audio|PlaySoundatLocation (Utilities|Select :Index (Variables|/Script/PhysicsCore.PhysicalMaterial|GetSurfaceType _physmat) :SurfaceType_Default (Variables|HitscanWeaponConfig|GetHitscanDefaultImpactSound) :SurfaceType1 (Variables|HitscanWeaponConfig|GetHitscanCharacterImpactSound)) _impactpoint "0, 0, 0" 1.0 1.0 0.0 0 0 0)
      (Effects|SpawnEmitteratLocation (Utilities|Select :Index (Variables|/Script/PhysicsCore.PhysicalMaterial|GetSurfaceType _physmat) :SurfaceType_Default (Variables|HitscanWeaponConfig|GetHitscanDefaultImpactPS) :SurfaceType1 (Variables|HitscanWeaponConfig|GetHitscanCharacterImpactPS)) _impactpoint (Math|Conversions|RotationFromXVector _impactnormal)))))

(fn MultiFireWeaponFX
  (params (HitResult :type Hit%20Result%20Structure) (Hit :type Boolean%20%28by%20ref%29))
  (bind (_bblockinghit _binitialoverlap _time _distance _location _impactpoint _normal _impactnormal _physmat) (Collision|BreakHitResult HitResult))
  (if (Variables|HitscanWeaponConfig|GetIsHitScanWeapon?)
    (if Hit
      ;[1 1 1] Play Impact Particle & Sound Based On Pysical Material
      (Audio|PlaySoundatLocation (Utilities|Select :Index (Variables|/Script/PhysicsCore.PhysicalMaterial|GetSurfaceType _physmat) :SurfaceType_Default (Variables|HitscanWeaponConfig|GetHitscanDefaultImpactSound) :SurfaceType1 (Variables|HitscanWeaponConfig|GetHitscanCharacterImpactSound)) _impactpoint "0, 0, 0" 1.0 1.0 0.0 0 0 0)
      (Effects|SpawnEmitteratLocation (Utilities|Select :Index (Variables|/Script/PhysicsCore.PhysicalMaterial|GetSurfaceType _physmat) :SurfaceType_Default (Variables|HitscanWeaponConfig|GetHitscanDefaultImpactPS) :SurfaceType1 (Variables|HitscanWeaponConfig|GetHitscanCharacterImpactPS)) _impactpoint (Math|Conversions|RotationFromXVector _impactnormal)))))

(fn StreamFireWeaponFX
  (params (HitResult :type Hit%20Result%20Structure) (Hit :type Boolean%20%28by%20ref%29))
  (bind (_bblockinghit _binitialoverlap _time _distance _location _impactpoint _normal _impactnormal _physmat) (Collision|BreakHitResult HitResult))
  ;[1 1 1] Play Firing Sound & Spawn Muzzle Flash (Sound Played Here Is For Not Auto Fire Weapons)
  (Effects|SpawnEmitterAttached (Variables|Effects|GetMuzzleFlashPS) (Variables|Default|GetWeaponMesh) (Variables|Default|GetMuzzleSocketName))
  (if (Variables|HitscanWeaponConfig|GetIsHitScanWeapon?)
    (if Hit
      ;[1 1 1] Play Impact Particle & Sound Based On Pysical Material
      (Audio|PlaySoundatLocation (Utilities|Select :Index (Variables|/Script/PhysicsCore.PhysicalMaterial|GetSurfaceType _physmat) :SurfaceType_Default (Variables|HitscanWeaponConfig|GetHitscanDefaultImpactSound) :SurfaceType1 (Variables|HitscanWeaponConfig|GetHitscanCharacterImpactSound)) _impactpoint "0, 0, 0" 1.0 1.0 0.0 0 0 0)
      (Effects|SpawnEmitteratLocation (Utilities|Select :Index (Variables|/Script/PhysicsCore.PhysicalMaterial|GetSurfaceType _physmat) :SurfaceType_Default (Variables|HitscanWeaponConfig|GetHitscanDefaultImpactPS) :SurfaceType1 (Variables|HitscanWeaponConfig|GetHitscanCharacterImpactPS)) _impactpoint (Math|Conversions|RotationFromXVector _impactnormal)))))