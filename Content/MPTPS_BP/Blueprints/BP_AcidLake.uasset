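; BP_AcidLake is an acid hazard that deals repeated damage to BP_Char_Master characters inside its AcidDamageCollider.
; Begin and end overlap call the ServerStartDamage and ServerStopDamage events.
; Starting damages immediately and sets a looping timer on AcidDamage, which re-sets itself each pulse using the configured interval and amount.
; One function-name timer serves the whole lake, so any character exiting clears it.
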(event OnComponentBeginOverlap(AcidDamageCollider)
  (params (OverlappedComponent :type Primitive%20Component%20Object%20Reference) (OtherActor :type Actor%20Object%20Reference) (OtherComp :type Primitive%20Component%20Object%20Reference) (OtherBodyIndex :type Integer) (bFromSweep :type Boolean) (SweepResult :type Hit%20Result%20Structure%20%28by%20ref%29))
  (bind _asbp_char_master (Utilities|Casting|CastToBP_Char_Master OtherActor))
  (CallFunction|ServerStartDamage _asbp_char_master))

(event OnComponentEndOverlap(AcidDamageCollider)
  (params (OverlappedComponent :type Primitive%20Component%20Object%20Reference) (OtherActor :type Actor%20Object%20Reference) (OtherComp :type Primitive%20Component%20Object%20Reference) (OtherBodyIndex :type Integer))
  (bind _asbp_char_master (Utilities|Casting|CastToBP_Char_Master OtherActor))
  (CallFunction|ServerStopDamage _asbp_char_master))

(event Custom|ServerStartDamage
  (params (Player :type BP%20Char%20Master%20Object%20Reference))
  (CallFunction|AcidDamage))

(event Custom|ServerStopDamage
  (params (Player :type BP%20Char%20Master%20Object%20Reference))
  (Utilities|Time|ClearTimerbyFunctionName 0 "AcidDamage"))

(event Custom|AcidDamage
  (Utilities|Time|SetTimerbyFunctionName 0 "AcidDamage" (Variables|AcidDamage|GetAcidDamageInterval) true) ; Create Pulses for Damage
  (Game|Damage|ApplyDamage (stale Custom|ServerStartDamage Player) (Variables|AcidDamage|GetAcidDamageAmount) 0 self))

(fn ConstructionScript)