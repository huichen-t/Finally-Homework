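; Elevator platform actor that shuttles between its origin and a configurable end location, with motor, steam and start sounds.
; A timeline scaled by travel time lerps the platform; on finishing it waits a stop delay, then runs the opposite way.
; A safety collider sends it forward again if a BP_Char_Master overlaps during the return trip.
; The construction script can preview the end position in-editor.
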(event OnComponentBeginOverlap(SafetyCollider)
  (params (OverlappedComponent :type Primitive%20Component%20Object%20Reference) (OtherActor :type Actor%20Object%20Reference) (OtherComp :type Primitive%20Component%20Object%20Reference) (OtherBodyIndex :type Integer) (bFromSweep :type Boolean) (SweepResult :type Hit%20Result%20Structure%20%28by%20ref%29))
  (bind _elevatortimeline (Variables|Default|GetElevatorTimeline))
  (bind _motorloop_01_cue (Variables|Default|GetMotorLoop_01_Cue))
  ;[1 1 1] Reverses direction if collision occurs with Actor
  (Utilities|Casting|CastToBP_Char_Master OtherActor)
  (if (Components|Activation|IsActive _elevatortimeline)
    (if (Class|TimelineComponent|IsReversing _elevatortimeline)
      ;[1 1 1] Sets Elevator End Location - Stop Delay- Reversing
      (bind (_direction _elevatorup) (Timeline|ElevatorTimeline Play) ; Float Translation Curve
        (:Update
          (Transformation|SetRelativeLocation (Variables|Default|GetElevator) (Math|Vector|Lerp(Vector) "0, 0, 0" (Variables|ElevatorControls|GetEndLocation) _elevatorup) false false))
        (:Finished
          (Utilities|FlowControl|Sequence
            (:then_0
              (Utilities|FlowControl|Delay (Variables|ElevatorControls|GetStopDelay))
              (Utilities|FlowControl|Sequence
                (:then_0
                  ;;[1 1 1] Start/Stop Audio
                  (Audio|Components|Audio|Play (Variables|Default|GetPlatform_Start_02_Cue) 0.0))
                (:then_1
                  (switch Utilities|FlowControl|Switch|SwitchonETimelineDirection _direction
                    (:Forward
                      (CallFunction|ElevatorReverese))
                    (:Backward
                      (CallFunction|ElevatorForward)))
                  (Audio|Components|Audio|Play _motorloop_01_cue 0.0))))
            (:then_1
              (Audio|Components|Audio|Play (Variables|Default|GetSteamStop_01_01_Cue) 0.0)
              (Audio|Components|Audio|Stop _motorloop_01_cue))))))))

(event Custom|ElevatorForward
  (bind _motorloop_01_cue (Variables|Default|GetMotorLoop_01_Cue))
  ;[1 1 1] Sets Elevator End Location - Stop Delay- Reversing
  ;;[1 1 1] Reverses direction if collision occurs with Actor
  (bind (_direction _elevatorup) (Timeline|ElevatorTimeline PlayFromStart) ; Float Translation Curve
    (:Update
      (Transformation|SetRelativeLocation (Variables|Default|GetElevator) (Math|Vector|Lerp(Vector) "0, 0, 0" (Variables|ElevatorControls|GetEndLocation) _elevatorup) false false))
    (:Finished
      (Utilities|FlowControl|Sequence
        (:then_0
          (Utilities|FlowControl|Delay (Variables|ElevatorControls|GetStopDelay))
          (Utilities|FlowControl|Sequence
            (:then_0
              ;;[1 1 1] Start/Stop Audio
              (Audio|Components|Audio|Play (Variables|Default|GetPlatform_Start_02_Cue) 0.0))
            (:then_1
              (switch Utilities|FlowControl|Switch|SwitchonETimelineDirection _direction
                (:Forward
                  (CallFunction|ElevatorReverese))
                (:Backward
                  (CallFunction|ElevatorForward)))
              (Audio|Components|Audio|Play _motorloop_01_cue 0.0))))
        (:then_1
          (Audio|Components|Audio|Play (Variables|Default|GetSteamStop_01_01_Cue) 0.0)
          (Audio|Components|Audio|Stop _motorloop_01_cue))))))

(event Custom|ElevatorReverese
  (bind _motorloop_01_cue (Variables|Default|GetMotorLoop_01_Cue))
  ;[1 1 1] Sets Elevator End Location - Stop Delay- Reversing
  ;;[1 1 1] Reverses direction if collision occurs with Actor
  (bind (_direction _elevatorup) (Timeline|ElevatorTimeline ReverseFromEnd) ; Float Translation Curve
    (:Update
      (Transformation|SetRelativeLocation (Variables|Default|GetElevator) (Math|Vector|Lerp(Vector) "0, 0, 0" (Variables|ElevatorControls|GetEndLocation) _elevatorup) false false))
    (:Finished
      (Utilities|FlowControl|Sequence
        (:then_0
          (Utilities|FlowControl|Delay (Variables|ElevatorControls|GetStopDelay))
          (Utilities|FlowControl|Sequence
            (:then_0
              ;;[1 1 1] Start/Stop Audio
              (Audio|Components|Audio|Play (Variables|Default|GetPlatform_Start_02_Cue) 0.0))
            (:then_1
              (switch Utilities|FlowControl|Switch|SwitchonETimelineDirection _direction
                (:Forward
                  (CallFunction|ElevatorReverese))
                (:Backward
                  (CallFunction|ElevatorForward)))
              (Audio|Components|Audio|Play _motorloop_01_cue 0.0))))
        (:then_1
          (Audio|Components|Audio|Play (Variables|Default|GetSteamStop_01_01_Cue) 0.0)
          (Audio|Components|Audio|Stop _motorloop_01_cue))))))

(event EventBeginPlay
  ;[1 1 1] Sets Travel Speed
  (Components|Timeline|SetPlayRate (Variables|Default|GetElevatorTimeline) (/ 1.0 (Variables|ElevatorControls|GetTravelTimeInSeconds)))
  (Variables|ElevatorControls|SetEndLocationPreview true) ; Safety to Defeat Test during Play
)

(fn ConstructionScript
  (Transformation|SetRelativeLocation (Variables|Default|GetElevator) (Math|Vector|SelectVector (Variables|ElevatorControls|GetEndLocation) "0, 0, 0" (Variables|ElevatorControls|GetEndLocationPreview)) false false))