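; Conquest-mode capture point that teams take by outnumbering each other inside its sphere, earning team points once captured.
; A one-second looping timer counts overlapping characters per team and uses the difference to drain the rival's counter, then build the leader's.
; At the threshold it reports the holder and awards points on each qualifying tick through FPS_Conquest_GS.
; Flag and decal materials switch between Team A, Team B and neutral.
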(event OnComponentEndOverlap(Sphere)
  (params (OverlappedComponent :type Primitive%20Component%20Object%20Reference) (OtherActor :type Actor%20Object%20Reference) (OtherComp :type Primitive%20Component%20Object%20Reference) (OtherBodyIndex :type Integer))
  ;[1 1 1] On End Overlap
  (bind _asbp_base_character (Utilities|Casting|CastToBP_BaseCharacter OtherActor))
  (Variables|/Game/FPS/Blueprints/CharacterAndClasses/BP_BaseCharacter.BP_BaseCharacter_C|SetbCapturingPoint _asbp_base_character false))

(event OnComponentBeginOverlap(Sphere)
  (params (OverlappedComponent :type Primitive%20Component%20Object%20Reference) (OtherActor :type Actor%20Object%20Reference) (OtherComp :type Primitive%20Component%20Object%20Reference) (OtherBodyIndex :type Integer) (bFromSweep :type Boolean) (SweepResult :type Hit%20Result%20Structure%20%28by%20ref%29))
  ;[1 0.581 0.966] OnBeginOverlap
  (Utilities|IsValid OtherActor
    (:Is%20Valid
      (bind _asbp_base_character (Utilities|Casting|CastToBP_BaseCharacter OtherActor))
      (Variables|Default|SetbCaptured true)
      (Variables|Default|SetbHolderTeam (Variables|/Game/FPS/Blueprints/CharacterAndClasses/BP_BaseCharacter.BP_BaseCharacter_C|GetbPawnTeam _asbp_base_character)))))

(event Custom|Increase%20Team%20Points
  (bind _pointstocapture (Variables|Default|GetPointsToCapture))
  (bind _gamestateref (Variables|Default|GetGameStateRef))
  (bind _gamestateref_2 (Variables|Default|GetGameStateRef))
  (bind _pointstocapture_2 (Variables|Default|GetPointsToCapture))
  ;[0.6962 0.3326 1] Flag Update
  (CallFunction|GetPlayersInside)
  (if (Variables|Default|GetbCaptured)
    (if (!= (Variables|Default|GetTeamAPlayers) (Variables|Default|GetTeamBPlayers))
      (if (> (Variables|Default|GetTeamAPlayers) (Variables|Default|GetTeamBPlayers))
        (Variables|Default|SetbHolderTeam false :!label _label)
        (if (== (Variables|Default|GetTeamBCounter) 0)
          (bind _output_get (Variables|Default|SetTeamACounter (+ (Variables|Default|GetTeamACounter) (Math|Integer|Absolute(Integer) (- (Variables|Default|GetTeamAPlayers) (Variables|Default|GetTeamBPlayers))))))
          (Default|SetCapturePointsProgess (Variables|Default|GetGameStateRef) (Variables|Default|GetPointId) (Utilities|Struct|MakeCapturePointInfo "NewEnumerator2" (Math|Integer|Clamp(Integer) _output_get 0 _pointstocapture) false))
          (if (>= (Math|Integer|Clamp(Integer) _output_get 0 _pointstocapture) _pointstocapture)
            (Default|AddTeamPoints _gamestateref false)
            (Default|SetCapturePointHolder _gamestateref false (Variables|Default|GetPointId))
            (Rendering|Components|Decal|SetDecalMaterial (Variables|Default|GetDecal) "/Game/FPS/Core/CapturePoints/A_ConquesDecal_Inst.A_ConquesDecal_Inst")
            (Rendering|Material|SetMaterial (Variables|Default|GetFlag_01) 0 "/Game/FPS/Core/Materials/FlagMaterial_Inst1.FlagMaterial_Inst1")
            (Variables|Default|SetFlagState "NewEnumerator0"))
          (else
            (bind _output_get_2 (Variables|Default|SetTeamBCounter (Math|Integer|Clamp(Integer) (- (Variables|Default|GetTeamBCounter) (Math|Integer|Absolute(Integer) (- (Variables|Default|GetTeamAPlayers) (Variables|Default|GetTeamBPlayers)))) 0 (Variables|Default|GetPointsToCapture))))
            (Default|SetCapturePointsProgess (Variables|Default|GetGameStateRef) (Variables|Default|GetPointId) (Utilities|Struct|MakeCapturePointInfo "NewEnumerator2" (Math|Integer|Clamp(Integer) (- (Variables|Default|GetTeamBCounter) (Math|Integer|Absolute(Integer) (- (Variables|Default|GetTeamAPlayers) (Variables|Default|GetTeamBPlayers)))) 0 (Variables|Default|GetPointsToCapture)) true))
            (if (== _output_get_2 0)
              (Rendering|Components|Decal|SetDecalMaterial (Variables|Default|GetDecal) "/Game/FPS/Core/CapturePoints/N_ConquesDecal_Inst2.N_ConquesDecal_Inst2")
              (Rendering|Material|SetMaterial (Variables|Default|GetFlag_01) 0 "/Game/FPS/Core/Materials/FlagMaterial_Inst2.FlagMaterial_Inst2")
              (Variables|Default|SetFlagState "NewEnumerator2"))))
        (else
          (Variables|Default|SetbHolderTeam true :!label _label_2)
          (if (== (Variables|Default|GetTeamACounter) 0)
            (bind _output_get_3 (Variables|Default|SetTeamBCounter (+ (Variables|Default|GetTeamBCounter) (Math|Integer|Absolute(Integer) (- (Variables|Default|GetTeamAPlayers) (Variables|Default|GetTeamBPlayers))))))
            (Default|SetCapturePointsProgess (Variables|Default|GetGameStateRef) (Variables|Default|GetPointId) (Utilities|Struct|MakeCapturePointInfo "NewEnumerator2" (Math|Integer|Clamp(Integer) _output_get_3 0 _pointstocapture_2) true))
            (if (>= (Math|Integer|Clamp(Integer) _output_get_3 0 _pointstocapture_2) _pointstocapture_2)
              (Default|AddTeamPoints _gamestateref_2 true)
              (Default|SetCapturePointHolder _gamestateref_2 true (Variables|Default|GetPointId))
              (Rendering|Components|Decal|SetDecalMaterial (Variables|Default|GetDecal) "/Game/FPS/Core/CapturePoints/B_ConquesDecal_Inst1.B_ConquesDecal_Inst1")
              (Rendering|Material|SetMaterial (Variables|Default|GetFlag_01) 0 "/Game/FPS/Core/Materials/FlagMaterial_Inst.FlagMaterial_Inst")
              (Variables|Default|SetFlagState "NewEnumerator1"))
            (else
              (bind _output_get_4 (Variables|Default|SetTeamACounter (Math|Integer|Clamp(Integer) (- (Variables|Default|GetTeamACounter) (Math|Integer|Absolute(Integer) (- (Variables|Default|GetTeamAPlayers) (Variables|Default|GetTeamBPlayers)))) 0 (Variables|Default|GetPointsToCapture))))
              (Default|SetCapturePointsProgess (Variables|Default|GetGameStateRef) (Variables|Default|GetPointId) (Utilities|Struct|MakeCapturePointInfo "NewEnumerator2" _output_get_4 false))
              (if (== _output_get_4 0)
                (Rendering|Components|Decal|SetDecalMaterial (Variables|Default|GetDecal) "/Game/FPS/Core/CapturePoints/N_ConquesDecal_Inst2.N_ConquesDecal_Inst2")
                (Rendering|Material|SetMaterial (Variables|Default|GetFlag_01) 0 "/Game/FPS/Core/Materials/FlagMaterial_Inst2.FlagMaterial_Inst2")
                (Variables|Default|SetFlagState "NewEnumerator2"))))))
      (elif (not (Variables|Default|GetbHolderTeam))
        (goto _label)
        (else
          (goto _label_2))))))

(event EventBeginPlay
  ;[0.6962 0.3326 1] Flag Update
  (bind _asfps_conquest_gs (Utilities|Casting|CastToFPS_Conquest_GS (Game|GetGameState)))
  (Variables|Default|SetGameStateRef _asfps_conquest_gs)
  (Variables|Default|SetPointsToCapture (Variables|/Game/FPS/Blueprints/Game/Conquest/FPS_Conquest_GS.FPS_Conquest_GS_C|GetPointsToCapture _asfps_conquest_gs))
  (Utilities|Time|SetTimerbyEvent (delegate Custom|Increase%20Team%20Points) 1.0 true))

(fn ConstructionScript)

(fn GetPlayersInside
  (Variables|Default|SetTeamAPlayers 0)
  (Variables|Default|SetTeamBPlayers 0)
  (for _array_element (Collision|GetOverlappingActors (Variables|Default|GetSphere) "/Game/FPS/Blueprints/CharacterAndClasses/BP_BaseCharacter.BP_BaseCharacter_C" :!class /Script/Engine.PrimitiveComponent)
    (bind _asbp_base_character (Utilities|Casting|CastToBP_BaseCharacter _array_element))
    (Variables|/Game/FPS/Blueprints/CharacterAndClasses/BP_BaseCharacter.BP_BaseCharacter_C|SetbCapturingPoint _asbp_base_character true)
    (Variables|/Game/FPS/Blueprints/CharacterAndClasses/BP_BaseCharacter.BP_BaseCharacter_C|SetCapturePoint _asbp_base_character (Variables|Default|GetPointId))
    (if (Variables|/Game/FPS/Blueprints/CharacterAndClasses/BP_BaseCharacter.BP_BaseCharacter_C|GetbPawnTeam _asbp_base_character)
      (bind _result (Math|Integer|IncrementInt (Variables|Default|GetTeamBPlayers))
        (:%20%20
          (Variables|Default|SetTeamBPlayers _result)))
      (else
        (bind _result_2 (Math|Integer|IncrementInt (Variables|Default|GetTeamAPlayers))
          (:%20%20
            (Variables|Default|SetTeamAPlayers _result_2)))))))