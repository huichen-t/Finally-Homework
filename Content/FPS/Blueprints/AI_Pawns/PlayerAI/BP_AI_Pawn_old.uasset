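; AI-controlled FPS bot pawn that spawns with team and weapon setup, fights blackboard targets and can drop limited mines as a class skill.
; Shoot uses timers for fire rate and auto fire, while BotShoot multi-traces a random spread cone toward the Enemy, reducing damage per successive hit.
; AnyDamage applies safe-zone and friendly-fire rules; death updates bot count, kills and kill feed, drops weapon and ammo, then ragdolls and destroys the pawn.
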(event Custom|ServerSpawnMine
  (params (NewParam :type Transform))
  ;[0.8079 1 0.4961] Class Skill
  (Game|SpawnActorfromClass "/Game/FPS/Blueprints/Misc/Mine/BP_Mine.BP_Mine_C" NewParam "Undefined" 0 self))

(event EventBeginPlay
  ;[1 1 1] Begin play
  (Utilities|FlowControl|Delay 0.2)
  (Variables|Default|SetbWantsToRun false)
  (Variables|Default|SetInteractTime 2.0)
  (if (not (Variables|Default|GetbPawnTeam))
    _
    (else
      (Rendering|Material|SetMaterial (Variables|Character|GetMesh) 0 "/Game/FPS/Characters/Textures/Chr_FPS_D1_Mat_Blue.Chr_FPS_D1_Mat_Blue")))
  (Variables|/Script/Engine.CharacterMovementComponent|SetMaxWalkSpeed (Variables|Character|GetCharacterMovement) (Variables|Default|GetDefaultMovementSpeed))
  (CallFunction|ServerEquipWeapons))

(event EventAutoShoot
  ;[1 1 1] Shoot
  (if (not (Variables|Default|GetbRunning))
    (bind _canshoot (CallFunction|TrytoShoot))
    (if _canshoot
      (Default|Shoot (Variables|Default|GetCurrentWeapon))
      (Variables|Default|SetbCanShoot false)
      (Utilities|Time|SetTimerbyEvent (delegate EventResetCanShoot) (Variables|/Game/FPS/Blueprints/Weapons/BP_BaseWeapon.BP_BaseWeapon_C|GetTimeBetweenShoots (Variables|Default|GetCurrentWeapon)))
      (CallFunction|BotShoot))))

(event EventResetCanShoot
  ;[1 1 1] Shoot
  (Variables|Default|SetbCanShoot true))

(event EventTick
  (params (DeltaSeconds :type Float%20%28single-precision%29))
  (|CallParentFunction DeltaSeconds))

(event EventUseClassSkill
  (bind _returnvalue (Transformation|GetActorLocation))
  ;[0.8079 1 0.4961] Class Skill
  (if (!= (Variables|Default|GetTraps) 0)
    (bind _result (Math|Integer|DecrementInt (Variables|Default|GetTraps))
      (:%20%20
        (Variables|Default|SetTraps _result)
        (bind _outhit (Collision|LineTraceByChannel _returnvalue (+ _returnvalue (+ (* (Transformation|GetActorForwardVector) 1e+03) (* (Transformation|GetActorUpVector) -5e+02))) "TraceTypeQuery1" false 0 "None"))
        (CallFunction|ServerSpawnMine (Math|Conversions|ToTransform(Vector) (.location _outhit)))))))

(event Game|Damage|EventAnyDamage
  (params (Damage :type Float%20%28single-precision%29) (DamageType :type Damage%20Type%20Object%20Reference) (InstigatedBy :type Controller%20Object%20Reference) (DamageCauser :type Actor%20Object%20Reference))
  (bind _self self)
  (bind _healthcomponent (Variables|Default|GetHealthComponent))
  ;[1 1 1] Any Damage
  (if (and (not (Variables|Default|GetbDead)) (not (Variables|Default|GetbIsInSafeZone)))
    (CallFunction|Impact DamageCauser)
    (Variables|Default|SetDamageToDo Damage :!label _label)
    (bind _asbase_character_pc (Utilities|Casting|CastToBaseCharacterPC InstigatedBy)
      (:then
        (bind _asfps_gm (Utilities|Casting|CastToFPS_GM (Game|GetGameMode)))
        (if (Math|Boolean|Equal(Boolean) (Variables|/Game/FPS/Blueprints/PlayerController/BaseCharacterPC.BaseCharacterPC_C|GetTeam _asbase_character_pc) (Variables|Default|GetbPawnTeam))
          (if (Variables|/Game/FPS/Blueprints/Game/FPS_GM.FPS_GM_C|GetbFriendlyFire _asfps_gm)
            (Variables|Default|SetDamageToDo (* (Variables|Default|GetDamageToDo) (Variables|/Game/FPS/Blueprints/Game/FPS_GM.FPS_GM_C|GetFriendlyDmgMultiplier _asfps_gm)))
            (bind _output_get (Variables|/Game/FPS/Blueprints/HealthComponent/HealthComponent.HealthComponent_C|SetHP _healthcomponent (Math|Float|Clamp(Float) (- (Variables|/Game/FPS/Blueprints/HealthComponent/HealthComponent.HealthComponent_C|GetHP _healthcomponent) (Variables|Default|GetDamageToDo)) 0.0 (Variables|/Game/FPS/Blueprints/HealthComponent/HealthComponent.HealthComponent_C|GetMaxHP _healthcomponent)) :!label _label_2))
            (CallFunction|UpdateHP _output_get)
            (if (<= _output_get 0.0)
              (Variables|Default|SetbDead true)
              (Variables|Default|SetbCapturingPoint false)
              (bind _asfps_gs (Utilities|Casting|CastToFPS_GS (Game|GetGameState)))
              (Default|ReduceBotsAlive _asfps_gs (Variables|Default|GetbPawnTeam))
              (CallFunction|SendInfotoKillFeed _asbase_character_pc self)
              (bind _asbase_character_pc_2 (Utilities|Casting|CastToBaseCharacterPC InstigatedBy)
                (:then
                  (Default|AddKill _asbase_character_pc_2 _self))
                (:CastFailed
                  _))
              (CallFunction|OnDeath _self)))
          (else
            (goto _label_2))))
      (:CastFailed
        (goto _label_2)))
    (elif (== DamageCauser self)
      (goto _label))))

(event Collision|EventActorBeginOverlap
  (params (OtherActor :type Actor%20Object%20Reference)))

(event EventOnDeath
  (params (Dead_Actor :type BP%20Base%20Character%20Object%20Reference) (Instigator :type Player%20Controller%20Object%20Reference))
  ;[1 1 1] On_Death
  (CallFunction|DropPrimaryWeapon)
  (CallFunction|StopAutoShootTimer)
  (Variables|Default|SetbWantsToRun false)
  (bind _asfps_player_state (Utilities|Casting|CastToFPS_PlayerState (Variables|Default|GetPlayerState))
    (:then
      (Default|AddDeath _asfps_player_state))
    (:CastFailed
      _))
  (Variables|Default|SetbRunning false)
  (Utilities|Time|PauseTimerbyHandle (Variables|Default|GetAutoShootTimerHandle))
  (Pawn|Components|CharacterMovement|DisableMovement (Variables|/Script/Engine.Character|GetCharacterMovement Dead_Actor))
  (CallFunction|ServerRagdoll Dead_Actor)
  (CallFunction|DropAmmo)
  (CallFunction|DestroyWeapon)
  (Utilities|FlowControl|Delay 6.0)
  (Actor|DestroyActor))

(event EventStopShooting
  ;[1 1 1] Shoot
  ;;[1 1 1] Stop Shooting
  (Utilities|Time|PauseTimerbyHandle (Variables|Default|GetAutoShootTimerHandle)))

(event EventShoot
  (bind _currentweapon (Variables|Default|GetCurrentWeapon))
  ;[1 1 1] Shoot
  (if (Math|Boolean|ANDBoolean (not (Variables|Default|GetbReloading)) (Variables|Default|GetbCanShoot) (not (Variables|Default|GetbRunning)))
    (Utilities|IsValid _currentweapon
      (:Is%20Valid
        (if (Variables|/Game/FPS/Blueprints/Weapons/BP_BaseWeapon.BP_BaseWeapon_C|GetbSemi _currentweapon)
          _
          (else
            (bind _returnvalue (Utilities|Time|SetTimerbyEvent (delegate EventAutoShoot) (Variables|/Game/FPS/Blueprints/Weapons/BP_BaseWeapon.BP_BaseWeapon_C|GetTimeBetweenShoots _currentweapon) true))
            (Variables|Default|SetAutoShootTimerHandle _returnvalue))))
      (:Is%20Not%20Valid
        _))
    (bind _canshoot (CallFunction|TrytoShoot))
    (if _canshoot
      (Default|Shoot (Variables|Default|GetCurrentWeapon))
      (Variables|Default|SetbCanShoot false)
      (Utilities|Time|SetTimerbyEvent (delegate EventResetCanShoot) (Variables|/Game/FPS/Blueprints/Weapons/BP_BaseWeapon.BP_BaseWeapon_C|GetTimeBetweenShoots (Variables|Default|GetCurrentWeapon)))
      (CallFunction|BotShoot))))

(fn ConstructionScript
  (|CallParentFunction)
  (Variables|Default|SetPrimaryWeaponToSpawn "/Game/FPS/Blueprints/Weapons/BP_AssaultWeapon.BP_AssaultWeapon_C")
  (Variables|Default|SetSecondaryWeaponToSpawn "/Game/FPS/Blueprints/Weapons/BP_SecondaryWeaponTest.BP_SecondaryWeaponTest_C"))

(fn BotShoot
  (bind _self self)
  (bind _enemy (Variables|Default|GetEnemy))
  (bind _currentweapon (Variables|Default|GetCurrentWeapon))
  (bind _returnvalue (AI|GetBlackboard _self))
  (bind _meshfpp (Variables|/Game/FPS/Blueprints/Weapons/BP_BaseWeapon.BP_BaseWeapon_C|GetMeshFPP _currentweapon))
  (bind _returnvalue_2 (Transformation|GetWorldLocation _meshfpp))
  (bind _returnvalue_3 (AI|Components|Blackboard|GetValueasObject _returnvalue _enemy))
  (bind _asbp_base_character (Utilities|Casting|CastToBP_BaseCharacter _returnvalue_3))
  (Utilities|IsValid _returnvalue_3
    (:Is%20Valid
      (if (not (Variables|/Game/FPS/Blueprints/CharacterAndClasses/BP_BaseCharacter.BP_BaseCharacter_C|GetbDead _asbp_base_character))
        (bind _outhits (Collision|MultiLineTraceByChannel _returnvalue_2 (+ _returnvalue_2 (* (Class|KismetMathLibrary|RandomUnitVectorinConeinRadians (Math|Vector|GetUnitDirection(Vector) _returnvalue_2 (Transformation|GetActorLocation _asbp_base_character)) (Variables|Default|GetBotWeaponSpread)) 6e+03)) "TraceTypeQuery3" false 0 "None"))
        (for (_array_element _array_index) _outhits
          (CallFunction|ServerPlayImpact "0, 0, 0" (.PhysMat (Collision|BreakHitResult _array_element)) (.ImpactNormal (Collision|BreakHitResult _array_element)))
          (Utilities|IsValid (.HitActor (Collision|BreakHitResult _array_element))
            (:Is%20Valid
              (Utilities|IsValid (Actor|GetComponentbyClass (.HitActor (Collision|BreakHitResult _array_element)) "/Game/FPS/Blueprints/HealthComponent/HealthComponent.HealthComponent_C")
                (:Is%20Valid
                  (CallFunction|ServerHit _array_element self (/ 1.0 (Math|Conversions|ToFloat(Integer) (+ _array_index 1)))))))))
        (Default|LocalPlayEffects (Variables|Default|GetCurrentWeapon))
        (CallFunction|PlayFPPShootEffects (.Location (Collision|BreakHitResult _array_element)))
        (else
          (AI|Components|Blackboard|SetValueasObject _returnvalue _enemy 0 :!label _label)
          (CallFunction|StopShooting))))
    (:Is%20Not%20Valid
      (goto _label))))